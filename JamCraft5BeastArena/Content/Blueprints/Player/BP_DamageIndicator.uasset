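; BP_DamageIndicator is a floating damage number actor that shows a rounded Value as world-space text, sized larger for higher values.
; On BeginPlay it picks a random target point above its spawn location and sets the text and size.
; Each tick it turns to face the first player's control rotation, eases toward the target with VInterpTo, and lowers text alpha by a fixed, frame-rate-dependent step until it destroys itself.
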(event EventBeginPlay
  (bind _textrender (Variables|Default|GetTextRender))
  (Variables|Default|SetMoveLocation (+ (Math|Vector|MakeVector (Math|Random|RandomFloatinRange -5e+01 5e+01) (Math|Random|RandomFloatinRange -5e+01 5e+01) (Math|Random|RandomFloatinRange 1.5e+02 2.5e+02)) (Transformation|GetActorLocation)))
  (Rendering|Components|TextRender|SetWorldSize _textrender (+ (* 12 (Variables|Default|GetValue)) 3e+01))
  (Rendering|Components|TextRender|SetText _textrender (Utilities|Text|ToText(String) (Class|KismetMathLibrary|Round64 (Variables|Default|GetValue)))))

(event EventTick
  (params (DeltaSeconds :type Float%20%28single-precision%29))
  (bind _returnvalue (Game|GetPlayerController 0))
  (bind _textrender (Variables|Default|GetTextRender))
  (bind _textrender_2 (Variables|Default|GetTextRender))
  (bind _returnvalue_2 (Pawn|GetControlRotation _returnvalue :!class /Script/Engine.Controller))
  (bind _textrendercolor (Variables|/Script/Engine.TextRenderComponent|GetTextRenderColor _textrender_2))
  (Transformation|SetWorldRotation _textrender (Math|Rotator|MakeRotator (.roll _returnvalue_2) (* (.pitch _returnvalue_2) -1.0) (+ (.yaw _returnvalue_2) 1.8e+02)) false false)
  (Rendering|Components|TextRender|SetTextRenderColor _textrender (Math|Color|MakeColor (.b _textrendercolor) (.g _textrendercolor) (.r _textrendercolor) (- (.a _textrendercolor) 5)))
  (Transformation|SetActorLocation (Math|Interpolation|VInterpTo (Transformation|GetActorLocation) (Variables|Default|GetMoveLocation) (Utilities|Time|GetWorldDeltaSeconds) 5.0) false false)
  (if (<= (.a _textrendercolor) 0)
    (Actor|DestroyActor)))

(fn ConstructionScript)