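; BP_Door is a double door that swings open when a BP_EnemyBase actor begins overlapping it and swings back when one leaves.
; A DoorOpen timeline, scaled by MaxAngle, drives the yaw of both panels in mirrored directions, with the left offset by 180 degrees.
; A DoOnce gate blocks repeated play calls until the timeline finishes, while end overlap reverses the timeline directly.
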(event Collision|EventActorBeginOverlap
  (params (OtherActor :type Actor%20Object%20Reference))
  (Utilities|Casting|CastToBP_EnemyBase OtherActor)
  (Utilities|FlowControl|DoOnce false :!label _label
    (:Completed
      (bind _rotation (Timeline|DoorOpen Play)
        (:Update
          (Transformation|SetRelativeRotation (Variables|Default|GetDoorRight) (Math|Rotator|MakeRotator 0.0 0.0 (* _rotation (Variables|Default|GetMaxAngle))) false false)
          (Transformation|SetRelativeRotation (Variables|Default|GetDoorLeft) (Math|Rotator|MakeRotator 0.0 0.0 (+ (* (* _rotation (Variables|Default|GetMaxAngle)) -1.0) 1.8e+02)) false false))
        (:Finished
          (goto _label Reset))))))

(event Collision|EventActorEndOverlap
  (params (OtherActor :type Actor%20Object%20Reference))
  (Utilities|Casting|CastToBP_EnemyBase OtherActor)
  (bind _rotation (Timeline|DoorOpen Reverse)
    (:Update
      (Transformation|SetRelativeRotation (Variables|Default|GetDoorRight) (Math|Rotator|MakeRotator 0.0 0.0 (* _rotation (Variables|Default|GetMaxAngle))) false false)
      (Transformation|SetRelativeRotation (Variables|Default|GetDoorLeft) (Math|Rotator|MakeRotator 0.0 0.0 (+ (* (* _rotation (Variables|Default|GetMaxAngle)) -1.0) 1.8e+02)) false false))
    (:Finished
      (Utilities|FlowControl|DoOnce false) ; enters at Reset
    )))

(fn ConstructionScript)