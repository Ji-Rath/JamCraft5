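; Base pickup item whose mesh, name and stats come from an ItemStructure variable, with the mesh also applied in the construction script.
; A name label shows while BP_Player overlaps the item, and Tick keeps it at the mesh location, facing back along the control rotation.
; Interacting passes the item data to the player's AddToInventory, randomizing durability below the structure's value, and destroys the actor if that succeeds.
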(event EventBeginPlay
  (bind _itemstructure (Variables|Default|GetItemStructure))
  (Components|StaticMesh|SetStaticMesh (Variables|Default|GetStaticMesh) (.mesh _itemstructure))
  (Rendering|Components|TextRender|SetText (Variables|Default|GetTextRender) (.name _itemstructure)))

(event Collision|EventActorBeginOverlap
  (params (OtherActor :type Actor%20Object%20Reference))
  (Utilities|Casting|CastToBP_Player OtherActor)
  (Rendering|SetVisibility (Variables|Default|GetTextRender) true false))

(event EventInteracted
  (bind _itemstructure (Variables|Default|GetItemStructure))
  (bind _asbp_player (Utilities|Casting|CastToBP_Player (Game|GetPlayerCharacter 0)))
  (bind _success (Default|AddtoInventory _asbp_player (Utilities|Struct|MakeItemStructure (.name _itemstructure) (.description _itemstructure) (.thumbnail _itemstructure) (.mesh _itemstructure) (.animation _itemstructure) (.class _itemstructure) (.damage _itemstructure) (.weapontype _itemstructure) (.isrighthand _itemstructure) (Math|Random|RandomInteger (.durability _itemstructure)))))
  (if _success
    (Actor|DestroyActor)))

(event Collision|EventActorEndOverlap
  (params (OtherActor :type Actor%20Object%20Reference))
  (Rendering|SetVisibility (Variables|Default|GetTextRender) false false))

(event EventTick
  (params (DeltaSeconds :type Float%20%28single-precision%29))
  (bind _returnvalue (Game|GetPlayerController 0))
  (bind _returnvalue_2 (Pawn|GetControlRotation _returnvalue :!class /Script/Engine.Controller))
  (if (Rendering|IsVisible (Variables|Default|GetTextRender))
    (Transformation|SetWorldRotation (Variables|Default|GetTextRender) (Math|Rotator|MakeRotator (.roll _returnvalue_2) (* (.pitch _returnvalue_2) -1.0) (+ (.yaw _returnvalue_2) 1.8e+02)) false false)
    (Transformation|SetWorldLocation (Variables|Default|GetTextRender) (Transformation|GetWorldLocation (Variables|Default|GetStaticMesh)) false false)))

(fn ConstructionScript
  (Components|StaticMesh|SetStaticMesh (Variables|Default|GetStaticMesh) (.mesh (Variables|Default|GetItemStructure))))