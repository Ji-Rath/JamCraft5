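; Bomb item that, once live, explodes after a short delay or on hitting anything not of the player's class.
; Tick spawns attached Niagara effects until detonation, which damages BP_EnemyBase actors overlapping the Sphere.
; A line trace only places hit effects and damage indicators, without gating damage.
; Mesh visibility guards against repeat blasts; the bomb spawns a destructible, hides, then destroys itself.
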(event EventBeginPlay)

(event EventTick
  (params (DeltaSeconds :type Float%20%28single-precision%29))
  (bind _returnvalue (Transformation|GetActorLocation))
  (bind _itemstructure (Variables|Default|GetItemStructure))
  (bind _staticmesh (Variables|Default|GetStaticMesh))
  (bind _returnvalue_2 (Rendering|IsVisible _staticmesh))
  (if (Variables|Default|GetIsLive)
    (if (not (Variables|Default|GetExploded))
      (Niagara|SpawnSystemAttached "/Game/Assets/Effects/Systems/Hit_System.Hit_System" (Variables|Default|GetStaticMesh) "None" "0, 0, 0" "0, 0, 0" "KeepRelativeOffset" true))
    (Utilities|FlowControl|Delay 2.5)
    (for _array_element (Collision|GetOverlappingActors (Variables|Default|GetSphere) "/Game/Blueprints/Enemies/BP_EnemyBase.BP_EnemyBase_C" :!class /Script/Engine.PrimitiveComponent)
      (if _returnvalue_2
        (Class|IsDamageable|TakeDamage(Message) _array_element (.damage _itemstructure))
        (bind (_outhit _returnvalue_3) (Collision|LineTraceByChannel _returnvalue (Transformation|GetActorLocation _array_element) "TraceTypeQuery3" true 0 "None" false))
        (if _returnvalue_3
          (Niagara|SpawnSystematLocation "/Game/Assets/Effects/Systems/Test_System.Test_System" (.Location (Collision|BreakHitResult _outhit)) (Math|Rotator|FindLookatRotation _returnvalue (.Location (Collision|BreakHitResult _outhit))))
          (Game|SpawnActorfromClass "/Game/Blueprints/Player/BP_DamageIndicator.BP_DamageIndicator_C" (Math|Conversions|ToTransform(Vector) (.Location (Collision|BreakHitResult _outhit))) "AlwaysSpawn" 0 (.damage _itemstructure) 0)
          (Components|Activation|Activate (Variables|Default|GetNiagara) false))))
    (if _returnvalue_2
      (Game|SpawnActorfromClass "/Game/Assets/Enemies/DestructableBP.DestructableBP_C" (Transformation|GetActorTransform) "AlwaysSpawn" 0 "/Game/Assets/Items/Weapons_Bomb_DM.Weapons_Bomb_DM" 0))
    (Rendering|SetVisibility (Variables|Default|GetStaticMesh) false false)
    (Variables|Default|SetExploded true)
    (Utilities|FlowControl|Delay 2.0)
    (Actor|DestroyActor)))

(event Collision|EventHit
  (params (MyComp :type Primitive%20Component%20Object%20Reference) (Other :type Actor%20Object%20Reference) (OtherComp :type Primitive%20Component%20Object%20Reference) (bSelfMoved :type Boolean) (HitLocation :type Vector :default "0, 0, 0") (HitNormal :type Vector :default "0, 0, 0") (NormalImpulse :type Vector :default "0, 0, 0") (Hit :type Hit%20Result%20Structure%20%28by%20ref%29))
  (bind _returnvalue (Transformation|GetActorLocation))
  (bind _itemstructure (Variables|Default|GetItemStructure))
  (bind _staticmesh (Variables|Default|GetStaticMesh))
  (bind _returnvalue_2 (Rendering|IsVisible _staticmesh))
  (if (and (!= (Utilities|GetClass Other) (Utilities|GetClass (Game|GetPlayerCharacter 0))) (Variables|Default|GetIsLive))
    (for _array_element (Collision|GetOverlappingActors (Variables|Default|GetSphere) "/Game/Blueprints/Enemies/BP_EnemyBase.BP_EnemyBase_C" :!class /Script/Engine.PrimitiveComponent)
      (if _returnvalue_2
        (Class|IsDamageable|TakeDamage(Message) _array_element (.damage _itemstructure))
        (bind (_outhit _returnvalue_3) (Collision|LineTraceByChannel _returnvalue (Transformation|GetActorLocation _array_element) "TraceTypeQuery3" true 0 "None" false))
        (if _returnvalue_3
          (Niagara|SpawnSystematLocation "/Game/Assets/Effects/Systems/Test_System.Test_System" (.Location (Collision|BreakHitResult _outhit)) (Math|Rotator|FindLookatRotation _returnvalue (.Location (Collision|BreakHitResult _outhit))))
          (Game|SpawnActorfromClass "/Game/Blueprints/Player/BP_DamageIndicator.BP_DamageIndicator_C" (Math|Conversions|ToTransform(Vector) (.Location (Collision|BreakHitResult _outhit))) "AlwaysSpawn" 0 (.damage _itemstructure) 0)
          (Components|Activation|Activate (Variables|Default|GetNiagara) false))))
    (if _returnvalue_2
      (Game|SpawnActorfromClass "/Game/Assets/Enemies/DestructableBP.DestructableBP_C" (Transformation|GetActorTransform) "AlwaysSpawn" 0 "/Game/Assets/Items/Weapons_Bomb_DM.Weapons_Bomb_DM" 0))
    (Rendering|SetVisibility (Variables|Default|GetStaticMesh) false false)
    (Variables|Default|SetExploded true)
    (Utilities|FlowControl|Delay 2.0)
    (Actor|DestroyActor)))

(fn ConstructionScript
  (|CallParentFunction))