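; Wave-based arena game mode that shows the title widget on BeginPlay and runs rounds of enemies and item drops.
; RoundCheck, when no enemies remain, starts a delayed SpawnEnemies timer and a looping SpawnItems timer that launches random items from spawn points up to the round's ItemCount.
; SpawnEnemies reads RoundInfo, places enemies at random spawn points scaled up by round to full size, falls back to the last entry for endless rounds, then increments Round.
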(event Custom|Round%20Check
  (bind _outactors (Actor|GetAllActorsOfClass "/Game/Blueprints/Enemies/BP_EnemyBase.BP_EnemyBase_C"))
  (if (== (Utilities|Array|Length _outactors) 0)
    (bind _returnvalue (Utilities|Time|SetTimerbyFunctionName 0 "SpawnEnemies" 15.0))
    (Variables|Default|SetSpawnTimer _returnvalue)
    (bind _returnvalue_2 (Utilities|Time|SetTimerbyFunctionName 0 "SpawnItems" 0.25 true 1.0))
    (Variables|Default|SetSpawnItemTimer _returnvalue_2)))

(event EventBeginPlay
  (bind _returnvalue (UserInterface|CreateWidget "/Game/Blueprints/UI/Title.Title_C"))
  (UserInterface|Viewport|AddtoViewport _returnvalue 0)
  (Variables|Default|SetTitleWidget _returnvalue)
  (bind _outactors (Actor|GetAllActorsOfClass "/Game/Blueprints/Enemies/BP_EnemyBase.BP_EnemyBase_C"))
  (if (== (Utilities|Array|Length _outactors) 0)
    (bind _returnvalue_2 (Utilities|Time|SetTimerbyFunctionName 0 "SpawnEnemies" 15.0))
    (Variables|Default|SetSpawnTimer _returnvalue_2)
    (bind _returnvalue_3 (Utilities|Time|SetTimerbyFunctionName 0 "SpawnItems" 0.25 true 1.0))
    (Variables|Default|SetSpawnItemTimer _returnvalue_3)))

(fn ConstructionScript)

(fn SpawnEnemies
  (bind _roundinfo (Variables|Default|GetRoundInfo))
  (bind _round (Variables|Default|GetRound))
  (bind _returnvalue (* _round 0.1))
  (bind _returnvalue_2 (+ _returnvalue 0.5))
  (bind _returnvalue_3 (Math|Float|Clamp(Float) _returnvalue_2 0.0 1.0))
  ;[1 1 1] Spawn Enemies
  (bind _outactors (Actor|GetAllActorsOfClass "/Game/Blueprints/Enemies/BP_SpawnPoint.BP_SpawnPoint_C"))
  (if (Utilities|Array|IsValidIndex _roundinfo _round)
    (for _array_element (.enemyarray (Utilities|Array|Get(acopy) _roundinfo _round))
      (Game|SpawnActorfromClass _array_element (Math|Transform|MakeTransform (Transformation|GetActorLocation (Utilities|Array|Get(acopy) _outactors (Math|Random|RandomInteger (Utilities|Array|Length _outactors)))) "0, 0, 0" (Math|Vector|MakeVector _returnvalue_3 _returnvalue_3 _returnvalue_3)) "AdjustIfPossibleButAlwaysSpawn" 0 (.Health (Utilities|GetClassDefaults _array_element)) 0))
    (else
      ;[1 1 1] Infinite Rounds
      (for _array_element_2 (.enemyarray (Utilities|Array|Get(acopy) _roundinfo (Utilities|Array|LastIndex _roundinfo)))
        (Game|SpawnActorfromClass _array_element (Math|Transform|MakeTransform (Transformation|GetActorLocation (Utilities|Array|Get(acopy) _outactors (Math|Random|RandomInteger (Utilities|Array|Length _outactors)))) "0, 0, 0" (Math|Vector|MakeVector _returnvalue_3 _returnvalue_3 _returnvalue_3)) "AdjustIfPossibleButAlwaysSpawn" 0 (.Health (Utilities|GetClassDefaults _array_element)) 0))))
  (Math|Integer|IncrementInt (Variables|Default|GetRound)))

(fn SpawnItems
  (bind _itemclass (Variables|Default|GetItemClass))
  ;[1 1 1] Spawn Items
  (if (< (Variables|Default|GetSpawnItemIndex) (.itemcount (Utilities|Array|Get(acopy) (Variables|Default|GetRoundInfo) (Variables|Default|GetRound))))
    (bind _outactors (Actor|GetAllActorsOfClass "/Game/Blueprints/Items/BP_ItemSpawnPoint.BP_ItemSpawnPoint_C"))
    (bind _output_get (Variables|Default|SetItemSpawn (Utilities|Array|Get(acopy) _outactors (Math|Random|RandomInteger (Utilities|Array|Length _outactors)))))
    (bind _returnvalue (Game|SpawnActorfromClass :Class (Utilities|Array|Get(acopy) _itemclass (Math|Random|RandomInteger (Utilities|Array|Length _itemclass))) :SpawnTransform (Transformation|GetActorTransform _output_get) :CollisionHandlingOverride "AlwaysSpawn" :Instigator 0))
    (Physics|AddImpulse (Variables|/Game/Blueprints/Items/BP_ItemBase.BP_ItemBase_C|GetStaticMesh _returnvalue) (* (Math|Vector|GetForwardVector (Transformation|GetActorRotation _output_get)) 5e+02) "None" true)
    (Math|Integer|IncrementInt (Variables|Default|GetSpawnItemIndex))
    (else
      (Utilities|Time|ClearandInvalidateTimerbyHandle (Variables|Default|GetSpawnItemTimer))
      (Variables|Default|SetSpawnItemIndex 0))))