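; BP_Spectator is a spectator actor that periodically throws a random item toward the player.
; BeginPlay picks an item class from rock, metal scrap, stick, empty flask, gunpowder or bomb.
; Tick waits on a random Delay, then spawns the item, launches it toward BP_Player with an upward impulse and attaches a trail effect.
; The IsBeingThrown flag then makes Tick re-roll the item before the next wait.
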(event EventTick
  (params (DeltaSeconds :type Float%20%28single-precision%29))
  (bind _returnvalue (Transformation|GetActorTransform))
  (if (Variables|Default|GetIsBeingThrown)
    (Variables|Default|SetIsBeingThrown false)
    (switch int (Math|Random|RandomInteger 6)
      (:Default
        (Variables|Default|SetItem "/Game/Blueprints/Items/BP_Rock.BP_Rock_C" :!label _label))
      (:0
        (goto _label))
      (:1
        (Variables|Default|SetItem "/Game/Blueprints/Items/BP_MetalScrap.BP_MetalScrap_C"))
      (:2
        (Variables|Default|SetItem "/Game/Blueprints/Items/BP_Stick.BP_Stick_C"))
      (:3
        (Variables|Default|SetItem "/Game/Blueprints/Items/BP_EmptyFlask.BP_EmptyFlask_C"))
      (:4
        (Variables|Default|SetItem "/Game/Blueprints/Items/BP_Stick.BP_Stick_C"))
      (:5
        (Variables|Default|SetItem "/Game/Blueprints/Items/BP_GunPowder.BP_GunPowder_C"))
      (:6
        (Variables|Default|SetItem "/Game/Blueprints/Items/BP_Bomb.BP_Bomb_C")))
    (else
      (bind _returnvalue_2 (Actor|GetActorOfClass "/Game/Blueprints/Player/BP_Player.BP_Player_C"))
      (Utilities|FlowControl|Delay (Math|Random|RandomFloatinRange 2e+01 6e+01))
      (bind _returnvalue_3 (Game|SpawnActorfromClass (Variables|Default|GetItem) (Math|Transform|MakeTransform (+ (.location _returnvalue) (* (Math|Vector|MakeVector (.X (Math|Vector|BreakVector (Math|Vector|GetForwardVector (Math|Rotator|FindLookatRotation (.location _returnvalue) (Transformation|GetActorLocation _returnvalue_2))))) (.Y (Math|Vector|BreakVector (Math|Vector|GetForwardVector (Math|Rotator|FindLookatRotation (.location _returnvalue) (Transformation|GetActorLocation _returnvalue_2))))) (+ (.Z (Math|Vector|BreakVector (Math|Vector|GetForwardVector (Math|Rotator|FindLookatRotation (.location _returnvalue) (Transformation|GetActorLocation _returnvalue_2))))) 1e+01)) 1e+02)) (.rotation _returnvalue)) "AlwaysSpawn" 0 (Utilities|GetClassDefaults (Variables|Default|GetItem)) 0))
      (Physics|AddImpulse (Variables|/Game/Blueprints/Items/BP_ItemBase.BP_ItemBase_C|GetStaticMesh _returnvalue_3) (Math|Vector|MakeVector (.x (* (Math|Vector|GetForwardVector (Math|Rotator|FindLookatRotation (.location _returnvalue) (Transformation|GetActorLocation _returnvalue_2))) 5e+02)) (.y (* (Math|Vector|GetForwardVector (Math|Rotator|FindLookatRotation (.location _returnvalue) (Transformation|GetActorLocation _returnvalue_2))) 5e+02)) (+ (.z (* (Math|Vector|GetForwardVector (Math|Rotator|FindLookatRotation (.location _returnvalue) (Transformation|GetActorLocation _returnvalue_2))) 5e+02)) 5e+02)) "None" true)
      (Niagara|SpawnSystemAttached "/Game/Assets/Effects/Systems/AttackTrail_System.AttackTrail_System" (Variables|/Game/Blueprints/Items/BP_ItemBase.BP_ItemBase_C|GetStaticMesh _returnvalue_3) "None" "0, 0, 0" "0, 0, 0" "KeepRelativeOffset" true)
      (Variables|Default|SetIsBeingThrown true))))

(event EventBeginPlay
  (switch int (Math|Random|RandomInteger 6)
    (:Default
      (Variables|Default|SetItem "/Game/Blueprints/Items/BP_Rock.BP_Rock_C" :!label _label))
    (:0
      (goto _label))
    (:1
      (Variables|Default|SetItem "/Game/Blueprints/Items/BP_MetalScrap.BP_MetalScrap_C"))
    (:2
      (Variables|Default|SetItem "/Game/Blueprints/Items/BP_Stick.BP_Stick_C"))
    (:3
      (Variables|Default|SetItem "/Game/Blueprints/Items/BP_EmptyFlask.BP_EmptyFlask_C"))
    (:4
      (Variables|Default|SetItem "/Game/Blueprints/Items/BP_Stick.BP_Stick_C"))
    (:5
      (Variables|Default|SetItem "/Game/Blueprints/Items/BP_GunPowder.BP_GunPowder_C"))
    (:6
      (Variables|Default|SetItem "/Game/Blueprints/Items/BP_Bomb.BP_Bomb_C"))))

(fn ConstructionScript)