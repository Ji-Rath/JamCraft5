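; Spectator actor that lobs a random item toward the ThirdPersonCharacter every 20 to 60 seconds.
; BeginPlay picks the first item class, and Tick runs a Delay, then spawns it with an upward-arcing impulse and attack trail.
; IsBeingThrown makes the following Tick pick the next item from rock, scrap, stick, flask or gunpowder.
; The Bomb case is unreachable because RandomInteger(6) only yields 0 to 5.
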(event EventTick
  (params (DeltaSeconds :type Float%20%28single-precision%29))
  (bind _returnvalue (Transformation|GetActorTransform))
  (if (Variables|Default|GetIsBeingThrown)
    (Variables|Default|SetIsBeingThrown false)
    (switch int (Math|Random|RandomInteger 6)
      (:Default
        (Variables|Default|SetItem "/Game/Blueprints/Items/Rock.Rock_C" :!label _label))
      (:0
        (goto _label))
      (:1
        (Variables|Default|SetItem "/Game/Blueprints/Items/MetalScrap.MetalScrap_C"))
      (:2
        (Variables|Default|SetItem "/Game/Blueprints/Items/Stick.Stick_C"))
      (:3
        (Variables|Default|SetItem "/Game/Blueprints/Items/EmptyFlask.EmptyFlask_C"))
      (:4
        (Variables|Default|SetItem "/Game/Blueprints/Items/Stick.Stick_C"))
      (:5
        (Variables|Default|SetItem "/Game/Blueprints/Items/Gunpowder.Gunpowder_C"))
      (:6
        (Variables|Default|SetItem "/Game/Blueprints/Items/Bomb.Bomb_C")))
    (else
      (bind _returnvalue_2 (Actor|GetActorOfClass "/Game/Blueprints/Player/ThirdPersonCharacter.ThirdPersonCharacter_C"))
      (Utilities|FlowControl|Delay (Math|Random|RandomFloatinRange 2e+01 6e+01))
      (bind _returnvalue_3 (Game|SpawnActorfromClass (Variables|Default|GetItem) (Math|Transform|MakeTransform (+ (.location _returnvalue) (* (Math|Vector|MakeVector (.X (Math|Vector|BreakVector (Math|Vector|GetForwardVector (Math|Rotator|FindLookatRotation (.location _returnvalue) (Transformation|GetActorLocation _returnvalue_2))))) (.Y (Math|Vector|BreakVector (Math|Vector|GetForwardVector (Math|Rotator|FindLookatRotation (.location _returnvalue) (Transformation|GetActorLocation _returnvalue_2))))) (+ (.Z (Math|Vector|BreakVector (Math|Vector|GetForwardVector (Math|Rotator|FindLookatRotation (.location _returnvalue) (Transformation|GetActorLocation _returnvalue_2))))) 1e+01)) 1e+02)) (.rotation _returnvalue)) "AlwaysSpawn" 0 (Utilities|GetClassDefaults (Variables|Default|GetItem)) 0))
      (Physics|AddImpulse (Variables|/Game/Blueprints/Items/Item.Item_C|GetStaticMesh _returnvalue_3) (Math|Vector|MakeVector (.x (* (Math|Vector|GetForwardVector (Math|Rotator|FindLookatRotation (.location _returnvalue) (Transformation|GetActorLocation _returnvalue_2))) 5e+02)) (.y (* (Math|Vector|GetForwardVector (Math|Rotator|FindLookatRotation (.location _returnvalue) (Transformation|GetActorLocation _returnvalue_2))) 5e+02)) (+ (.z (* (Math|Vector|GetForwardVector (Math|Rotator|FindLookatRotation (.location _returnvalue) (Transformation|GetActorLocation _returnvalue_2))) 5e+02)) 5e+02)) "None" true)
      (Niagara|SpawnSystemAttached "/Game/Assets/Effects/NiagaraSystem/AttackTrail_System.AttackTrail_System" (Variables|/Game/Blueprints/Items/Item.Item_C|GetStaticMesh _returnvalue_3) "None" "0, 0, 0" "0, 0, 0" "KeepRelativeOffset" true)
      (Variables|Default|SetIsBeingThrown true))))

(event EventBeginPlay
  (switch int (Math|Random|RandomInteger 6)
    (:Default
      (Variables|Default|SetItem "/Game/Blueprints/Items/Rock.Rock_C" :!label _label))
    (:0
      (goto _label))
    (:1
      (Variables|Default|SetItem "/Game/Blueprints/Items/MetalScrap.MetalScrap_C"))
    (:2
      (Variables|Default|SetItem "/Game/Blueprints/Items/Stick.Stick_C"))
    (:3
      (Variables|Default|SetItem "/Game/Blueprints/Items/EmptyFlask.EmptyFlask_C"))
    (:4
      (Variables|Default|SetItem "/Game/Blueprints/Items/Stick.Stick_C"))
    (:5
      (Variables|Default|SetItem "/Game/Blueprints/Items/Gunpowder.Gunpowder_C"))
    (:6
      (Variables|Default|SetItem "/Game/Blueprints/Items/Bomb.Bomb_C"))))

(fn ConstructionScript)