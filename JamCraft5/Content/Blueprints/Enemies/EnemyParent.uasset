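; Base enemy Blueprint that scales health with capsule size, damages actors through IsDamageable and knocks back the player.
; AttackCheck fires a radial impulse, damages overlapping actors and calls KnockBackPlayer, which launches players unless already knocked up or dodging.
; KnockSideways is a lateral launch variant that also deals damage.
; On death it spawns a destructible, destroys itself, triggers the game mode's round check and randomly plays crowd cheers.
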(event Custom|AttackCheck
  (params (BoxCheck :type Box%20Component%20Object%20Reference))
  (Class|RadialForceComponent|FireImpulse (Variables|Default|GetRadialForce))
  (for _array_element (Collision|GetOverlappingActors BoxCheck 0 :!class /Script/Engine.PrimitiveComponent)
    (if (and (Utilities|DoesObjectImplementInterface _array_element "/Game/Blueprints/IsDamageable.IsDamageable_C") (!= _array_element self))
      (Class|IsDamageable|TakeDamage(Message) _array_element 5.0)
      (CallFunction|KnockBackPlayer 0 5e+02))))

(event EventBeginPlay
  (bind _output_get (Variables|Default|SetHealth (+ (* (+ (.x (Transformation|GetWorldScale (Variables|Collision|GetCapsuleComponent))) 0.5) (Variables|Default|GetHealth)) 5.0)))
  (Variables|Default|SetMaxHealth _output_get))

(event Collision|EventActorBeginOverlap
  (params (OtherActor :type Actor%20Object%20Reference)))

(event EventTakeDamage
  (params (Amount :type Float%20%28single-precision%29))
  (Variables|Default|SetHealth (- (Variables|Default|GetHealth) Amount))
  (if (<= (Variables|Default|GetHealth) 0.0)
    (Game|SpawnActorfromClass "/Game/Assets/Enemies/DestructableBP.DestructableBP_C" (Transformation|GetActorTransform) "AlwaysSpawn" 0 (Variables|Default|GetDestructable) 0)
    (Actor|DestroyActor)
    (bind _asthird_person_game_mode (Utilities|Casting|CastToThirdPersonGameMode (Game|GetGameMode)))
    (Default|RoundCheck _asthird_person_game_mode)
    (if (Math|Random|RandomBool)
      (Audio|PlaySound2D (select (Math|Random|RandomBool) "/Game/Assets/Sound/Effects/crowdcheer.crowdcheer" "/Game/Assets/Sound/Effects/crowdcheer2.crowdcheer2") 1.0 1.0 0.0 0 0))))

(event EventTick
  (params (DeltaSeconds :type Float%20%28single-precision%29)))

(fn ConstructionScript)

(fn KnockBackPlayer
  (params (Actor :type Actor%20Object%20Reference) (Magnitude :type Float%20%28single-precision%29))
  (for _array_element (Collision|GetOverlappingActors (Variables|Default|GetBox) 0 :!class /Script/Engine.PrimitiveComponent)
    (bind _asthird_person_character (Utilities|Casting|CastToThirdPersonCharacter _array_element))
    (if (and (not (or (Animation|Montage|MontageIsPlaying (Components|SkeletalMesh|GetAnimInstance (Variables|/Script/Engine.Character|GetMesh _asthird_person_character)) "/Game/Assets/Player/Animations/PlayerKnockedUp.PlayerKnockedUp") (Animation|Montage|MontageIsPlaying (Components|SkeletalMesh|GetAnimInstance (Variables|/Script/Engine.Character|GetMesh _asthird_person_character)) "/Game/Assets/Player/Animations/PlayerDodge.PlayerDodge"))) (!= _asthird_person_character self))
      (Character|LaunchCharacter _asthird_person_character (Math|Vector|MakeVector (.x (* (Math|Vector|GetForwardVector (Math|Rotator|FindLookatRotation (Transformation|GetWorldLocation (Variables|Collision|GetCapsuleComponent)) (Transformation|GetWorldLocation (Variables|/Script/Engine.Character|GetCapsuleComponent _asthird_person_character)))) Magnitude)) (.y (* (Math|Vector|GetForwardVector (Math|Rotator|FindLookatRotation (Transformation|GetWorldLocation (Variables|Collision|GetCapsuleComponent)) (Transformation|GetWorldLocation (Variables|/Script/Engine.Character|GetCapsuleComponent _asthird_person_character)))) Magnitude)) 2.5e+02) true true)
      (Animation|Montage|MontagePlay (Components|SkeletalMesh|GetAnimInstance (Variables|/Script/Engine.Character|GetMesh _asthird_person_character)) "/Game/Assets/Player/Animations/PlayerKnockedUp.PlayerKnockedUp" 1.0 "MontageLength" 0.0 true)
      (if (and (Math|Random|RandomBool) (Math|Random|RandomBool))
        (Audio|PlaySound2D (select (Math|Random|RandomBool) "/Game/Assets/Sound/Effects/crowdyell.crowdyell" "/Game/Assets/Sound/Effects/crowdgasp.crowdgasp") 1.0 1.0 0.0 0 0)))))

(fn KnockSideways
  (params (Actor :type Actor%20Object%20Reference) (Magnitude :type Float%20%28single-precision%29))
  (bind _returnvalue (Pawn|GetControlRotation :!class /Script/Engine.Pawn))
  (bind _returnvalue_2 (Math|Vector|GetRightVector _returnvalue))
  (bind _returnvalue_3 (Math|Vector|ClampVectorSize _returnvalue_2 -1.0 1.0))
  (bind _returnvalue_4 (* _returnvalue_3 Magnitude))
  (for _array_element (Collision|GetOverlappingActors (Variables|Default|GetFrontBox) 0 :!class /Script/Engine.PrimitiveComponent)
    (bind _asthird_person_character (Utilities|Casting|CastToThirdPersonCharacter _array_element))
    (if (and (not (or (Animation|Montage|MontageIsPlaying (Components|SkeletalMesh|GetAnimInstance (Variables|/Script/Engine.Character|GetMesh _asthird_person_character)) "/Game/Assets/Player/Animations/PlayerKnockedUp.PlayerKnockedUp") (Animation|Montage|MontageIsPlaying (Components|SkeletalMesh|GetAnimInstance (Variables|/Script/Engine.Character|GetMesh _asthird_person_character)) "/Game/Assets/Player/Animations/PlayerDodge.PlayerDodge"))) (!= _asthird_person_character self))
      (Character|LaunchCharacter _asthird_person_character (Math|Vector|MakeVector (.x _returnvalue_4) (.y _returnvalue_4) 2.5e+02) true true)
      (Animation|Montage|MontagePlay (Components|SkeletalMesh|GetAnimInstance (Variables|/Script/Engine.Character|GetMesh _asthird_person_character)) "/Game/Assets/Player/Animations/PlayerKnockedUp.PlayerKnockedUp" 1.0 "MontageLength" 0.0 true)
      (Default|TakeDamage _asthird_person_character 5.0))))