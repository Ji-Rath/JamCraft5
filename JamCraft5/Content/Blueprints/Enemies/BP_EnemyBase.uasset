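; Base arena enemy Blueprint that handles scale-based health, death and melee knockback against the player.
; Health grows with capsule scale; at zero the enemy is replaced by a destructible, the game mode runs RoundCheck, and spectators animate with crowd audio.
; AttackCheck fires a radial impulse, then damages and launches an overlapping player away, skipping those dodging or already knocked up.
; KnockSideways instead launches players in FrontBox along the control rotation's right vector.
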(event EventBeginPlay
  (bind _output_get (Variables|Default|SetHealth (+ (* (+ (.x (Transformation|GetWorldScale (Variables|Collision|GetCapsuleComponent))) 0.5) (Variables|Default|GetHealth)) 5.0)))
  (Variables|Default|SetMaxHealth _output_get))

(event EventTakeDamage
  (params (Amount :type Float%20%28single-precision%29))
  (Variables|Default|SetHealth (- (Variables|Default|GetHealth) Amount))
  (if (<= (Variables|Default|GetHealth) 0.0)
    (Actor|DestroyActor)
    (Game|SpawnActorfromClass "/Game/Assets/Enemies/DestructableBP.DestructableBP_C" (Transformation|GetActorTransform) "AlwaysSpawn" 0 (Variables|Default|GetDestructable) 0)
    (bind _asarena_game_mode (Utilities|Casting|CastToArenaGameMode (Game|GetGameMode)))
    (Default|RoundCheck _asarena_game_mode)
    (bind _outactors (Actor|GetAllActorsOfClass "/Game/Blueprints/Spectator/BP_Spectator.BP_Spectator_C"))
    (for _array_element _outactors
      (bind _asspectator_skeleton_anim_blueprint (Utilities|Casting|CastToSpectator_Skeleton_AnimBlueprint (Components|SkeletalMesh|GetAnimInstance (Variables|/Game/Blueprints/Spectator/BP_Spectator.BP_Spectator_C|GetSkeletalMesh _array_element))))
      (Default|PlayAnimation _asspectator_skeleton_anim_blueprint))
    (Audio|PlaySound2D "/Game/Assets/Sound/Cue/S_Crowd_Cue.S_Crowd_Cue" 1.0 1.0 0.0 0 0)))

(fn ConstructionScript)

(fn KnockBackPlayer
  (params (Actor :type Actor%20Object%20Reference) (Magnitude :type Float%20%28single-precision%29))
  (bind _asbp_player (Utilities|Casting|CastToBP_Player Actor))
  (LocalVariables|SetPlayerRef _asbp_player)
  (Character|LaunchCharacter (LocalVariables|GetPlayerRef) (Math|Vector|MakeVector (.x (* (Math|Vector|GetForwardVector (Math|Rotator|FindLookatRotation (Transformation|GetActorLocation) (Transformation|GetActorLocation (LocalVariables|GetPlayerRef)))) Magnitude)) (.y (* (Math|Vector|GetForwardVector (Math|Rotator|FindLookatRotation (Transformation|GetActorLocation) (Transformation|GetActorLocation (LocalVariables|GetPlayerRef)))) Magnitude)) 2.5e+02) true true)
  (Animation|Montage|MontagePlay (Variables|/Game/Blueprints/Player/BP_Player.BP_Player_C|GetPlayerAnimInstance (LocalVariables|GetPlayerRef)) "/Game/Assets/Player/Animations/PlayerKnockedUp.PlayerKnockedUp" 1.0 "MontageLength" 0.0 true)
  (if (Math|Random|RandomBool)
    (Audio|PlaySound2D "/Game/Assets/Sound/Cue/S_Crowd_Cue.S_Crowd_Cue" 1.0 1.0 0.0 0 0)))

(fn KnockSideways
  (params (Actor :type Actor%20Object%20Reference) (Magnitude :type Float%20%28single-precision%29))
  (bind _returnvalue (Pawn|GetControlRotation :!class /Script/Engine.Pawn))
  (bind _returnvalue_2 (Math|Vector|GetRightVector _returnvalue))
  (bind _returnvalue_3 (Math|Vector|ClampVectorSize _returnvalue_2 -1.0 1.0))
  (bind _returnvalue_4 (* _returnvalue_3 Magnitude))
  (for _array_element (Collision|GetOverlappingActors (Variables|Default|GetFrontBox) 0 :!class /Script/Engine.PrimitiveComponent)
    (bind _asbp_player (Utilities|Casting|CastToBP_Player _array_element))
    (if (and (not (or (Animation|Montage|MontageIsPlaying (Components|SkeletalMesh|GetAnimInstance (Variables|/Script/Engine.Character|GetMesh _asbp_player)) "/Game/Assets/Player/Animations/PlayerKnockedUp.PlayerKnockedUp") (Animation|Montage|MontageIsPlaying (Components|SkeletalMesh|GetAnimInstance (Variables|/Script/Engine.Character|GetMesh _asbp_player)) "/Game/Assets/Player/Animations/PlayerDodge.PlayerDodge"))) (!= _asbp_player self))
      (Character|LaunchCharacter _asbp_player (Math|Vector|MakeVector (.x _returnvalue_4) (.y _returnvalue_4) 2.5e+02) true true)
      (Animation|Montage|MontagePlay (Components|SkeletalMesh|GetAnimInstance (Variables|/Script/Engine.Character|GetMesh _asbp_player)) "/Game/Assets/Player/Animations/PlayerKnockedUp.PlayerKnockedUp" 1.0 "MontageLength" 0.0 true)
      (Default|TakeDamage _asbp_player 5.0))))

(fn CanKnockback
  (params (Player :type Character%20Object%20Reference))
  (bind _mesh (Variables|/Script/Engine.Character|GetMesh Player))
  (bind _returnvalue (Components|SkeletalMesh|GetAnimInstance _mesh))
  (return (and (not (or (Animation|Montage|MontageIsPlaying _returnvalue "/Game/Assets/Player/Animations/PlayerDodge.PlayerDodge") (Animation|Montage|MontageIsPlaying _returnvalue "/Game/Assets/Player/Animations/PlayerKnockedUp.PlayerKnockedUp"))) (!= Player self))))

(fn AttackCheck
  (params (BoxCheck :type Box%20Component%20Object%20Reference) (Magnitude :type Float%20%28single-precision%29))
  (Class|RadialForceComponent|FireImpulse (Variables|Default|GetRadialForce))
  (for _array_element (Collision|GetOverlappingActors BoxCheck "/Script/Engine.Pawn" :!class /Script/Engine.PrimitiveComponent)
    (bind _asbp_player (Utilities|Casting|CastToBP_Player _array_element))
    (bind _returnvalue (CallFunction|CanKnockback _asbp_player))
    (if (Math|Boolean|ANDBoolean _returnvalue (Utilities|DoesObjectImplementInterface _array_element "/Game/Blueprints/IsDamageable.IsDamageable_C") (!= _array_element self) (> (Variables|/Game/Blueprints/Player/BP_Player.BP_Player_C|GetHealth _asbp_player) 0.0))
      (Class|IsDamageable|TakeDamage(Message) _array_element 5.0)
      (CallFunction|KnockBackPlayer _array_element Magnitude)
      (return true)))
  (return false))