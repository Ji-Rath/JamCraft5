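; BP_DamageIndicator is a floating damage number actor that pops up, shows a rounded Value and fades away.
; On BeginPlay it launches its capsule with a random upward impulse and sets text size and content from Value, so bigger hits show larger.
; Each Tick it turns the text toward the first player's view using the control rotation and lowers text alpha by a fixed step, destroying itself once invisible.
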(event EventBeginPlay
  (bind _textrender (Variables|Default|GetTextRender))
  (Physics|AddImpulse (Variables|Default|GetCapsule) (Math|Vector|MakeVector (Math|Random|RandomFloatinRange -1e+02 1e+02) (Math|Random|RandomFloatinRange -1e+02 1e+02) (Math|Random|RandomFloatinRange 3e+02 5e+02)) "None" false)
  (Rendering|Components|TextRender|SetWorldSize _textrender (+ (* 12 (Variables|Default|GetValue)) 3e+01))
  (Rendering|Components|TextRender|SetText _textrender (Utilities|Text|ToText(String) (Class|KismetMathLibrary|Round64 (Variables|Default|GetValue)))))

(event Collision|EventActorBeginOverlap
  (params (OtherActor :type Actor%20Object%20Reference)))

(event EventTick
  (params (DeltaSeconds :type Float%20%28single-precision%29))
  (bind _returnvalue (Game|GetPlayerController 0))
  (bind _textrender (Variables|Default|GetTextRender))
  (bind _returnvalue_2 (Pawn|GetControlRotation _returnvalue :!class /Script/Engine.Controller))
  (bind _textrendercolor (Variables|/Script/Engine.TextRenderComponent|GetTextRenderColor _textrender))
  (Transformation|SetWorldRotation _textrender (Math|Rotator|MakeRotator (.roll _returnvalue_2) (* (.pitch _returnvalue_2) -1.0) (+ (.yaw _returnvalue_2) 1.8e+02)) false false)
  (Rendering|Components|TextRender|SetTextRenderColor _textrender (Math|Color|MakeColor (.b _textrendercolor) (.g _textrendercolor) (.r _textrendercolor) (- (.a _textrendercolor) 5)))
  (if (<= (.a _textrendercolor) 0)
    (Actor|DestroyActor)))

(fn ConstructionScript)